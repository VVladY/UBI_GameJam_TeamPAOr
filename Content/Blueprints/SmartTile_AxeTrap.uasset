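; Smart tile axe trap that swings an axe and damages the player on contact.
; On BeginPlay the AxeSwing timeline offsets the Axe component's roll from the actor rotation cached in the Construction Script.
; An Axe hit on a FirstPersonCharacter passes a DoOnce that is never reset, so damage applies only once.
; The same hit spawns an explosion emitter, using the hit's NormalImpulse vector as its location.
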(event OnComponentHit(Axe)
  (params (OtherActor :type Actor%20Object%20Reference) (OtherComp :type Primitive%20Component%20Object%20Reference) (NormalImpulse :type Vector) (Hit :type Hit%20Result%20Structure%20%28by%20ref%29))
  (bind _asfirst_person_character (Utilities|Casting|CastToFirstPersonCharacter OtherActor))
  (Utilities|FlowControl|DoOnce false
    (:Completed
      (Game|Damage|ApplyDamage _asfirst_person_character (Variables|Default|GetAxeDamage) 0 0)
      (Effects|SpawnEmitteratLocation "/Game/StarterContent/Particles/P_Explosion.P_Explosion" NormalImpulse))))

(event EventBeginPlay
  (bind _initialrotation (Variables|Default|GetInitialRotation))
  (bind (_roll _pitch _yaw) (Math|Rotator|BreakRotator _initialrotation))
  (bind _axerotation (Timeline|AxeSwing Play)
    (:Update
      (Transformation|SetRelativeRotation (Variables|Default|GetAxe) (Math|Rotator|MakeRotator (+ _roll _axerotation) _pitch _yaw) false false))))

(fn ConstructionScript
  (bind _returnvalue (Transformation|GetActorRotation))
  (Transformation|SetActorRelativeRotation _returnvalue)
  (Variables|Default|SetInitialRotation _returnvalue))