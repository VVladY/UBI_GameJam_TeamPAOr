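; SmartTile is a self-spawning track tile actor that extends the level as the first-person character advances and removes itself afterwards.
; When the character overlaps EndTrigger, the tile asks FirstPersonGameMode to add another tile and starts checking GetTileDistance every Tick.
; Once that distance reaches a threshold, the tile destroys itself after a short delay.
; GetAttachTransform exposes the AttachPoint world transform.
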(event OnComponentBeginOverlap(EndTrigger)
  (params (OtherActor :type Actor%20Object%20Reference) (OtherComp :type Primitive%20Component%20Object%20Reference) (OtherBodyIndex :type Integer) (bFromSweep :type Boolean) (SweepResult :type Hit%20Result%20Structure%20%28by%20ref%29))
  (bind _asfirst_person_character (Utilities|Casting|CastToFirstPersonCharacter OtherActor))
  (bind _asfirst_person_game_mode (Utilities|Casting|CastToFirstPersonGameMode (Game|GetGameMode)))
  (Default|AddTile _asfirst_person_game_mode)
  (Variables|Default|SetHasSpawned true))

(event EventBeginPlay)

(event EventActorBeginOverlap
  (params (OtherActor :type Actor%20Object%20Reference)))

(event EventTick
  (params (DeltaSeconds :type Float%20%28single-precision%29)))

(event EventTick
  (params (DeltaSeconds :type Float%20%28single-precision%29))
  (if (Variables|Default|GetHasSpawned)
    (if (>= (|GetTileDistance (stale OnComponentBeginOverlap(EndTrigger) _asfirst_person_character)) 2e+03)
      (Variables|Default|SetHasSpawned false)
      (Utilities|FlowControl|Delay 0.2)
      (Actor|DestroyActor))))

(fn ConstructionScript)

(fn GetAttachTransform
  (return (Transformation|GetWorldTransform (Variables|Default|GetAttachPoint))))