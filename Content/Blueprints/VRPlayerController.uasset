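; VR player controller providing gaze-based interaction, a context menu and runtime headset and graphics tuning.
; A camera line trace finds "Interactive" components, whose tagged children highlight through dynamic materials or visibility while gaze time accumulates.
; ToggleMenu spawns or destroys the menu facing the camera, forcing sticky highlighting while open.
; Helpers apply screen percentage, distortion, IPD, vsync and scalability through console commands; screen percentage and distortion settings save to a slot.
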(fn ConstructionScript)

(fn ManuallyChangeScreenPercentage
  (Variables|HMDSettings|SetCurrentSP (Math|Float|Clamp(Float) (Variables|HMDSettings|GetCurrentSP) (Variables|HMDSettings|GetLowestSP) (Variables|HMDSettings|GetHighestSP)))
  (Development|ExecuteConsoleCommand (Utilities|String|Append "hmd sp " (Utilities|String|ToString(Float) (Variables|HMDSettings|GetCurrentSP)))))

(fn ManuallyChangeDistortionScale
  (Variables|HMDSettings|SetCurrentDistortionScale (Math|Float|Clamp(Float) (Variables|HMDSettings|GetCurrentDistortionScale) 0.2 2.0))
  (Development|ExecuteConsoleCommand (Utilities|String|Append (Utilities|String|Append (Utilities|String|Append "oculusdev on | " "hmdwarp 1=1 | ") "hmdwarp s=") (Utilities|String|ToString(Float) (Variables|HMDSettings|GetCurrentDistortionScale)))))

(fn CheckforInteractiveObjects
  (bind _returnvalue (Game|GetPlayerCameraManager 0))
  (bind _returnvalue_2 (Transformation|GetActorLocation _returnvalue))
  (bind (_outhit _returnvalue_3) (Collision|LineTraceForObjects _returnvalue_2 (+ _returnvalue_2 (* (Transformation|GetActorForwardVector _returnvalue) (Variables|HighlightingAndInteraction|GetInteractionDistance))) (Utilities|Array|MakeArray "ObjectTypeQuery2" "ObjectTypeQuery1" "ObjectTypeQuery4") false (Utilities|Array|MakeArray (Game|Player|GetPlayerPawn 0)) "None"))
  (if _returnvalue_3
    (Variables|Default|SetImpactPoint (.ImpactPoint (Collision|BreakHitResult _outhit)))
    (Variables|HighlightingAndInteraction|SetLookingAtComponent (.HitComponent (Collision|BreakHitResult _outhit))) ; Used For Un-Highlighting when DoesHighlight Stick Is off
    (return (Components|ComponentHasTag (.HitComponent (Collision|BreakHitResult _outhit)) "Interactive") (.HitComponent (Collision|BreakHitResult _outhit)) (.HitActor (Collision|BreakHitResult _outhit)))))

(fn HighlightInteractiveObject
  (params (LookingAtObject :type Primitive%20Component%20Object%20Reference))
  (if (== (Variables|HighlightingAndInteraction|GetHighlightedAmount) 0)
    (for _array_element (Components|GetChildrenComponents LookingAtObject true)
      (if (Components|ComponentHasTag _array_element "CanHighlight")
        (bind _asprimitive_component (Utilities|Casting|CastToPrimitiveComponent _array_element))
        (bind _returnvalue (Rendering|Material|CreateDynamicMaterialInstance _asprimitive_component 0 0 :!class /Script/Engine.PrimitiveComponent))
        (Rendering|Material|SetScalarParameterValue _returnvalue "HighlightedAmount" 1.0 :!class /Script/Engine.MaterialInstanceDynamic)
        (if (Components|ComponentHasTag _array_element "EffectedByTime")
          (Variables|HighlightingAndInteraction|SetHighlightedTimeChangingObject _array_element))
        (elif (Components|ComponentHasTag _array_element "ToggleOnView")
          (Rendering|SetVisibility _array_element true false))))
    (Variables|HighlightingAndInteraction|SetHighlightedObject LookingAtObject)
    (Variables|HighlightingAndInteraction|SetHighlightedAmount 1)
    (elif (Variables|HighlightingAndInteraction|GetDoesHighlightStick)
      (if (!= LookingAtObject (Variables|HighlightingAndInteraction|GetHighlightedObject))
        (for _array_element_2 (Components|GetChildrenComponents (Variables|HighlightingAndInteraction|GetHighlightedObject) true)
          (if (Components|ComponentHasTag _array_element_2 "CanHighlight")
            (bind _asprimitive_component_2 (Utilities|Casting|CastToPrimitiveComponent _array_element_2))
            (bind _returnvalue_2 (Rendering|Material|CreateDynamicMaterialInstance _asprimitive_component_2 0 0 :!class /Script/Engine.PrimitiveComponent))
            (Rendering|Material|SetScalarParameterValue _returnvalue_2 "HighlightedAmount" 0.0 :!class /Script/Engine.MaterialInstanceDynamic)
            (elif (Components|ComponentHasTag _array_element_2 "ToggleOnView")
              (Rendering|SetVisibility _array_element_2 false false))))
        (Variables|HighlightingAndInteraction|SetHighlightedAmount 0)
        (Variables|HighlightingAndInteraction|SetIsUpdateingTimeBaseMaterial false)
        (else
          (Variables|HighlightingAndInteraction|SetAmountOfTimeLookedAtObject (+ (Variables|HighlightingAndInteraction|GetAmountOfTimeLookedAtObject) (Variables|AutoSPVariables|GetDeltaSeconds)) :!label _label)
          (Variables|HighlightingAndInteraction|SetIsUpdateingTimeBaseMaterial true)))
      (else
        (goto _label)))))

(fn SaveHMDSettings
  (bind _ashmdsettings_save (Utilities|Casting|CastToHMDSettingsSave (Variables|Default|GetHMDSettingsSave)))
  (Variables|/Game/Blueprints/HMDSettingsSave.HMDSettingsSave_C|SetCurrentSP _ashmdsettings_save (Variables|HMDSettings|GetCurrentSP))
  (Variables|/Game/Blueprints/HMDSettingsSave.HMDSettingsSave_C|SetHighestSP _ashmdsettings_save (Variables|HMDSettings|GetHighestSP))
  (Variables|/Game/Blueprints/HMDSettingsSave.HMDSettingsSave_C|SetLowestSP _ashmdsettings_save (Variables|HMDSettings|GetLowestSP))
  (Variables|/Game/Blueprints/HMDSettingsSave.HMDSettingsSave_C|SetDistortionScale _ashmdsettings_save (Variables|HMDSettings|GetCurrentDistortionScale))
  (SaveGame|SaveGametoSlot (Variables|Default|GetHMDSettingsSave) "HMDSettings"))

(fn ToggleMenu
  (bind _returnvalue (Game|GetPlayerCameraManager 0))
  (bind _returnvalue_2 (Transformation|GetActorTransform _returnvalue))
  (bind _returnvalue_3 (Transformation|GetActorForwardVector _returnvalue))
  (bind (_location _rotation _scale) (Math|Transform|BreakTransform _returnvalue_2))
  (if (Variables|Default|GetIsMenuOpen)
    (Actor|DestroyActor (Variables|Default|GetCurrentlyOpenMenu))
    (Variables|Default|SetIsMenuOpen false)
    (Variables|HighlightingAndInteraction|SetDoesHighlightStick (Variables|Default|GetBeforeMenuHighlighting))
    (else
      (Variables|Default|SetBeforeMenuHighlighting (Variables|HighlightingAndInteraction|GetDoesHighlightStick))
      (bind _returnvalue_4 (Game|SpawnActorfromClass "/Game/Blueprints/ContextMenu.ContextMenu_C" (Math|Transform|MakeTransform (+ _location (* _returnvalue_3 1e+02)) (Math|Rotator|MakeRotfromXZ (* _returnvalue_3 -1.0) (Transformation|GetActorUpVector (Game|GetPlayerCharacter 0))) _scale) "AlwaysSpawn" 0 0))
      (Variables|Default|SetCurrentlyOpenMenu _returnvalue_4)
      (Variables|Default|SetIsMenuOpen true)
      (Variables|HighlightingAndInteraction|SetDoesHighlightStick true))))

(fn ManuallyChangeIPD
  (if (Variables|Default|GetIPDOverride)
    (Development|ExecuteConsoleCommand (Utilities|String|Append "stereo e=" (Utilities|String|ToString(Float) (/ (Variables|HMDSettings|GetCurrentIPD) 1e+03))))
    (else
      (Development|ExecuteConsoleCommand "stereo reset"))))

(fn ManuallyChangeVsync
  (if (Variables|Default|GetVsyncEnabled)
    (Development|ExecuteConsoleCommand "hmd vsync on")
    (else
      (Development|ExecuteConsoleCommand "hmd vsync Off"))))

(fn ManuallyChangeScalabilitySettings
  (Development|ExecuteConsoleCommand (Utilities|String|Append "sg.PostProcessQuality " (Utilities|String|ToString(Float) (Variables|ScalabilitySettings|GetCurrentPostProcessQuality))))
  (Development|ExecuteConsoleCommand (Utilities|String|Append "sg.ShadowQuality " (Utilities|String|ToString(Float) (Variables|ScalabilitySettings|GetCurrentShadowQuality))))
  (Development|ExecuteConsoleCommand (Utilities|String|Append "sg.TextureQuality " (Utilities|String|ToString(Float) (Variables|ScalabilitySettings|GetCurrentTextureQuality))))
  (Development|ExecuteConsoleCommand (Utilities|String|Append "sg.EffectsQuality " (Utilities|String|ToString(Float) (Variables|ScalabilitySettings|GetCurrentEffectsQuality))))
  (Development|ExecuteConsoleCommand (Utilities|String|Append "r.ViewDistanceScale " (Utilities|String|ToString(Float) (Math|Float|Clamp(Float) (Variables|ScalabilitySettings|GetCurrentViewDistanceScale) 0.1 2.0))))
  (Development|ExecuteConsoleCommand (Utilities|String|Append "r.PostProcessAAQuality " (Utilities|String|ToString(Float) (Math|Float|Clamp(Float) (Variables|ScalabilitySettings|GetCurrentAAQuality) 0.0 6.0)))))