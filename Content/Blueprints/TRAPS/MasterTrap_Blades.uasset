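; Master blade trap actor that slides a TrapDisc component along its local X axis while spinning it in pitch.
; On BeginPlay the Position timeline plays at DiscSpeedMovement, and each update calls Play on the Rotation timeline.
; Rotation updates combine both timeline values into the disc's relative transform, without sweeping.
; The construction script reapplies the actor's rotation and stores it as InitialRotation.
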(event EventBeginPlay
  (Components|Timeline|SetPlayRate (Variables|Default|GetPosition) (Variables|Default|GetDiscSpeedMovement))
  (bind _movement (Timeline|Position Play)
    (:Update
      (bind _rotation (Timeline|Rotation Play)
        (:Update
          (Transformation|SetRelativeTransform (Variables|Default|GetTrap_disc) (Math|Transform|MakeTransform (Math|Vector|MakeVector _movement 0.0 0.0) (Math|Rotator|MakeRotator 0.0 _rotation 0.0)) false false))))))

(fn ConstructionScript
  (bind _returnvalue (Transformation|GetActorRotation))
  (Transformation|SetActorRelativeRotation _returnvalue)
  (Variables|Default|SetInitialRotation _returnvalue))