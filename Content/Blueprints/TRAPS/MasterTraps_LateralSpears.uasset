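; Lateral spear trap that continuously launches Spear actors from random points within a box volume.
; Tick passes through a Gate with no open or close control into a short Delay, throttling spawns to a steady interval.
; Each spawn offsets the actor location by a random point in the scaled Box extents, ignoring box rotation.
; The Arrow component's world rotation sets the orientation of every spear.
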(event EventTick
  (params (DeltaSeconds :type Float%20%28single-precision%29))
  (bind _box (Variables|Default|GetBox))
  (bind _returnvalue (Components|Box|GetScaledBoxExtent _box))
  (bind (_x _y _z) (Math|Vector|BreakVector _returnvalue))
  (Utilities|FlowControl|Gate false
    (:Exit
      (Utilities|FlowControl|Delay 0.2)
      (Game|SpawnActorfromClass "/Game/FirstPersonBP/Blueprints/Spear.Spear_C" (Math|Transform|MakeTransform (+ (Math|Vector|MakeVector (Math|Random|RandomFloatinRange (* _x -1.0) _x) (Math|Random|RandomFloatinRange (* _y -1.0) _y) (Math|Random|RandomFloatinRange (* _z -1.0) _z)) (Transformation|GetActorLocation)) (Transformation|GetWorldRotation (Variables|Default|GetArrow)) "1.000000,1.000000,1.000000") "Undefined" 0 0))))

(fn ConstructionScript)