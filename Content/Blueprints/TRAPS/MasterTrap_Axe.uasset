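; Axe trap Blueprint that animates an axe component's roll using a timeline.
; The Construction Script caches the actor's rotation as InitialRotation.
; BeginPlay plays the timeline with AxeSpeed, adding its AxeRotation track to the cached roll and setting the result as the axe's relative rotation.
; The file has no overlap, damage or tick logic.
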(event EventBeginPlay
  (bind _initialrotation (Variables|Default|GetInitialRotation))
  (bind (_roll _pitch _yaw) (Math|Rotator|BreakRotator _initialrotation))
  (bind _axerotation (Timeline|Timeline_0 Play)
    (:Update
      (Transformation|SetRelativeRotation (Variables|Default|GetAxe) (Math|Rotator|MakeRotator (+ _roll _axerotation) _pitch _yaw) false false))))

(event EventActorBeginOverlap
  (params (OtherActor :type Actor%20Object%20Reference)))

(event EventTick
  (params (DeltaSeconds :type Float%20%28single-precision%29)))

(fn ConstructionScript
  (bind _returnvalue (Transformation|GetActorRotation))
  (Transformation|SetActorRelativeRotation _returnvalue)
  (Variables|Default|SetInitialRotation _returnvalue))