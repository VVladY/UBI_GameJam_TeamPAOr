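; Spear trap spawn volume that, once its Trigger is overlapped, continuously spawns random actors from ActorList.
; The overlap opens a Gate on Tick that is never closed here, and a short Delay throttles the spawn rate.
; Each spawn gets a random offset within the Box extent around the actor location, zero rotation and slight random per-axis scale.
; The random index range includes the list length, so it can land out of bounds.
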(event OnComponentBeginOverlap(trigger)
  (params (OtherActor :type Actor%20Object%20Reference) (OtherComp :type Primitive%20Component%20Object%20Reference) (OtherBodyIndex :type Integer) (bFromSweep :type Boolean) (SweepResult :type Hit%20Result%20Structure%20%28by%20ref%29))
  (bind _returnvalue (Math|Random|RandomFloatinRange 0.8 1.2))
  (bind _box (Variables|Default|GetBox))
  (bind _actorlist (Variables|Default|GetActorList))
  (bind _returnvalue_2 (Components|Box|GetScaledBoxExtent _box))
  (bind (_x _y _z) (Math|Vector|BreakVector _returnvalue_2))
  (Utilities|FlowControl|Gate true) ; enters at Open
)

(event Collision|EventActorBeginOverlap
  (params (OtherActor :type Actor%20Object%20Reference)))

(event EventTick
  (params (DeltaSeconds :type Float%20%28single-precision%29)))

(event EventTick
  (params (DeltaSeconds :type Float%20%28single-precision%29))
  (bind _returnvalue (Math|Random|RandomFloatinRange 0.8 1.2))
  (bind _box (Variables|Default|GetBox))
  (bind _actorlist (Variables|Default|GetActorList))
  (bind _returnvalue_2 (Components|Box|GetScaledBoxExtent _box))
  (bind (_x _y _z) (Math|Vector|BreakVector _returnvalue_2))
  (Utilities|FlowControl|Gate true
    (:Exit
      (Utilities|FlowControl|Delay 0.2)
      (Game|SpawnActorfromClass (Utilities|Array|Get(acopy) _actorlist (Math|Random|RandomIntegerinRange 0 (Utilities|Array|Length _actorlist))) (Math|Transform|MakeTransform (+ (Math|Vector|MakeVector (Math|Random|RandomFloatinRange (* _x -1.0) _x) (Math|Random|RandomFloatinRange (* _y -1.0) _y) (Math|Random|RandomFloatinRange (* _z -1.0) _z)) (Transformation|GetActorLocation)) "0, 0, 0" (Math|Vector|MakeVector _returnvalue _returnvalue _returnvalue)) "Undefined" 0 0))))

(fn ConstructionScript)