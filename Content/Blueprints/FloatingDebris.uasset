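; FloatingDebris is a short-lived destructible debris actor with a randomized look and thrust, which destroys itself 20 seconds after play begins.
; The construction script picks a random destructible mesh from an array, applies a material and gives its dynamic instance a random base color.
; It also randomizes the thrust strength of the Push component, so pieces differ in how hard they are propelled.
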(event EventBeginPlay
  (Utilities|FlowControl|Delay 2e+01)
  (Actor|DestroyActor))

(event EventActorBeginOverlap
  (params (OtherActor :type Actor%20Object%20Reference)))

(event EventTick
  (params (DeltaSeconds :type Float%20%28single-precision%29)))

(fn ConstructionScript
  (bind _mesh (Variables|Default|GetMesh))
  (bind _destructible (Variables|Default|GetDestructible))
  (Class|DestructibleComponent|SetDestructibleMesh _destructible (Utilities|Array|Get(acopy) _mesh (Math|Random|RandomInteger (Utilities|Array|Length _mesh))))
  (Rendering|Material|SetMaterial _destructible 0 (Variables|Default|GetMaterial))
  (bind _returnvalue (Rendering|Material|CreateDynamicMaterialInstance _destructible 0 0 :!class /Script/Engine.PrimitiveComponent))
  (Rendering|Material|SetVectorParameterValue _returnvalue "Base Color" (Utilities|Struct|MakeLinearColor (Math|Random|RandomFloatinRange 0.0 1.0) (Math|Random|RandomFloatinRange 0.0 1.0) (Math|Random|RandomFloatinRange 0.0 1.0) 1.0) :!class /Script/Engine.MaterialInstanceDynamic)
  (Variables|/Script/Engine.PhysicsThrusterComponent|SetThrustStrength (Variables|Default|GetPush) (Math|Random|RandomFloatinRange 1e+05 1e+06)))